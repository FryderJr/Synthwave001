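; BP_Platform is a track segment that drives platform spawning and cleanup as the player character crosses its Box trigger.
; On entry it calls PopulatePlatform on itself and asks BP_SynthwaveGameMode to add another platform.
; On exit it gives attached actors a short lifespan and itself a longer one, so passed segments destroy themselves.
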(event OnComponentBeginOverlap(Box)
  (params (OverlappedComponent :type Primitive%20Component%20Object%20Reference) (OtherActor :type Actor%20Object%20Reference) (OtherComp :type Primitive%20Component%20Object%20Reference) (OtherBodyIndex :type Integer) (bFromSweep :type Boolean) (SweepResult :type Hit%20Result%20Structure%20%28by%20ref%29))
  (Utilities|Casting|CastToSynthwave001Character OtherActor)
  (Class|GeneratedPlatform|PopulatePlatform)
  (bind _asbp_synthwave_game_mode (Utilities|Casting|CastToBP_SynthwaveGameMode (Game|GetGameMode)))
  (Class|Synthwave001GameMode|AddPlatform _asbp_synthwave_game_mode))

(event OnComponentEndOverlap(Box)
  (params (OverlappedComponent :type Primitive%20Component%20Object%20Reference) (OtherActor :type Actor%20Object%20Reference) (OtherComp :type Primitive%20Component%20Object%20Reference) (OtherBodyIndex :type Integer))
  (Utilities|Casting|CastToSynthwave001Character OtherActor)
  (for _array_element (Actor|GetAttachedActors true)
    (Actor|SetLifeSpan _array_element 1.0))
  (Actor|SetLifeSpan 7.5))

(event EventBeginPlay)

(event Collision|EventActorBeginOverlap
  (params (OtherActor :type Actor%20Object%20Reference)))

(event EventTick
  (params (DeltaSeconds :type Float%20%28single-precision%29)))

(fn ConstructionScript)