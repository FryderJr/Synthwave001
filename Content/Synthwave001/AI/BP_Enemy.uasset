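; BP_Enemy is an AI-controlled enemy that shows its health on an attached widget.
; On BeginPlay it stores its AI controller, runs the BT_Enemy behavior tree and binds to the HealthComponent's health-changed event.
; DisplayHealth pushes the current health into the WBP_EnemyHealth widget at startup and on every health change, so no Tick update is needed.
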(event Custom|OnHealthChanged_Event_0
  (params (HealthComp :type Health%20Component%20Object%20Reference) (Health :type Float%20%28single-precision%29) (HealthDelta :type Float%20%28single-precision%29) (DamageType :type Damage%20Type%20Object%20Reference) (InstigatedBy :type Controller%20Object%20Reference) (DamageCauser :type Actor%20Object%20Reference))
  (CallFunction|DisplayHealth))

(event EventBeginPlay
  (bind _self self)
  (bind _returnvalue (AI|GetAIController _self))
  (Variables|Default|SetCurrentController _returnvalue)
  (AI|RunBehaviorTree _returnvalue "/Game/Synthwave001/AI/BT_Enemy.BT_Enemy")
  (EventDispatchers|AssignOnHealthChanged (Variables|Default|GetHealthComponent) (delegate Custom|OnHealthChanged_Event_0))
  (CallFunction|DisplayHealth))

(event Collision|EventActorBeginOverlap
  (params (OtherActor :type Actor%20Object%20Reference)))

(event EventTick
  (params (DeltaSeconds :type Float%20%28single-precision%29)))

(fn ConstructionScript)

(fn DisplayHealth
  (bind _aswbp_enemy_health (Utilities|Casting|CastToWBP_EnemyHealth (UserInterface|GetUserWidgetObject (Variables|Default|GetWidget))))
  (Default|UpdateHealth _aswbp_enemy_health (Variables|/Script/Synthwave001.HealthComponent|GetHealth (Variables|Default|GetHealthComponent))))