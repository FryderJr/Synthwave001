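; BP_MeleeEnemy is an AI melee enemy that runs the BT_MeleeEnemy behavior tree on begin play.
; Its Health component drives a health widget and a hit flash made by stamping the damage time into a dynamic material parameter.
; At zero health it detaches from its controller and is removed after a short lifespan.
; An Attack event randomly plays one of two swing montages.
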(event OnHealthChanged(Health)
  (params (HealthComp :type Health%20Component%20Object%20Reference) (Health :type Float%20%28single-precision%29) (HealthDelta :type Float%20%28single-precision%29) (DamageType :type Damage%20Type%20Object%20Reference) (InstigatedBy :type Controller%20Object%20Reference) (DamageCauser :type Actor%20Object%20Reference))
  (CallFunction|Blink)
  (CallFunction|DisplayHealth)
  (if (<= Health 0.0)
    (Class|Pawn|DetachfromControllerPendingDestroy)
    (Actor|SetLifeSpan 1e+01)))

(event Custom|Attack
  (bind _mesh (Variables|Character|GetMesh))
  (switch int (Math|Random|RandomInteger 2)
    (:0
      (Animation|Montage|PlayMontage _mesh "/Game/Synthwave001/Character/Animations/StandingMeleeAttackHorizontal4UE4_Montage.StandingMeleeAttackHorizontal4UE4_Montage"))
    (:1
      (Animation|Montage|PlayMontage _mesh "/Game/Synthwave001/Character/Animations/StandingMeleeAttackBackhand4UE4_Montage.StandingMeleeAttackBackhand4UE4_Montage"))))

(event EventBeginPlay
  (CallFunction|DisplayHealth)
  (AI|RunBehaviorTree (AI|GetAIController self) "/Game/Synthwave001/AI/BT_MeleeEnemy.BT_MeleeEnemy"))

(event Collision|EventActorBeginOverlap
  (params (OtherActor :type Actor%20Object%20Reference)))

(event EventTick
  (params (DeltaSeconds :type Float%20%28single-precision%29)))

(fn ConstructionScript)

(fn DisplayHealth
  (bind _aswbp_enemy_health (Utilities|Casting|CastToWBP_EnemyHealth (UserInterface|GetUserWidgetObject (Variables|Default|GetWidget))))
  (Default|UpdateHealth _aswbp_enemy_health (Variables|/Script/Synthwave001.HealthComponent|GetHealth (Variables|Default|GetHealth))))

(fn Blink
  (bind _returnvalue (Rendering|Material|CreateDynamicMaterialInstance (Variables|Character|GetMesh) 0 (Utilities|Array|Get(acopy) (Rendering|Material|GetMaterials (Variables|Character|GetMesh))) "None" :!class /Script/Engine.PrimitiveComponent))
  (Rendering|Material|SetScalarParameterValue _returnvalue "LastTimeDamageTaken" (Utilities|Time|GetTimeSeconds) :!class /Script/Engine.MaterialInstanceDynamic))